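; BP_InteractiveHealth is an interactive health pickup that heals the player who interacts with it.
; Its Interact function adds HealValue through the player's AddHealth only when Health is below DefaultHealth, then destroys the actor.
; At full health the interaction does nothing, so the pickup stays in the world; the event graph holds only disabled stub events.
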(fn `Interact`
  (params (PlayerRef :type "/Game/BP/BP_FlowerPCharacter Object Reference"))
  (bind _playerref (`local.PlayerRef`))
  (if (not (>= (`/Game/BP/BP_FlowerPCharacter.Health` _playerref) (`/Game/BP/BP_FlowerPCharacter.DefaultHealth` _playerref)))
    (`/Game/BP/BP_FlowerPCharacter.AddHealth` (`local.PlayerRef`) (`self.Heal Value`))
    (`self.K2_DestroyActor`)))

(fn `UserConstructionScript`
  (`parent.UserConstructionScript`))