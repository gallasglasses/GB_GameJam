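; BP_InteractiveElevator is an interactive elevator that moves its PaperFlipbook while the flower player character is inside its InteractiveCollider.
; Overlap begin plays a timeline that lerps the flipbook's relative location between vectors A and B without sweeping.
; Overlap end stops the timeline without reversing, so the flipbook holds its position and playback resumes from there on re-entry.
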(event `self.InteractiveCollider.OnComponentBeginOverlap`
  (params (OverlappedComponent :type "PrimitiveComponent Object Reference") (OtherActor :type "Actor Object Reference") (OtherComp :type "PrimitiveComponent Object Reference") (OtherBodyIndex :type Integer) (bFromSweep :type Boolean) (SweepResult :type "HitResult Structure (by ref)"))
  (cast `/Game/BP/BP_FlowerPCharacter` OtherActor)
  (bind (_direction _newtrack_0) (`Timeline|Timeline_0` :!label _label)
    (:`Update`
      (`SceneComponent.K2_SetRelativeLocation` (`self.PaperFlipbook`) (`KismetMathLibrary.VLerp` (`self.A`) (`self.B`) _newtrack_0) false false))))

(event `self.InteractiveCollider.OnComponentEndOverlap`
  (params (OverlappedComponent :type "PrimitiveComponent Object Reference") (OtherActor :type "Actor Object Reference") (OtherComp :type "PrimitiveComponent Object Reference") (OtherBodyIndex :type Integer))
  (cast `/Game/BP/BP_FlowerPCharacter` OtherActor)
  (goto _label :!via `Stop`))

(fn `UserConstructionScript`
  (`parent.UserConstructionScript`))