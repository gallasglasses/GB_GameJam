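; BP_InteractiveSwitch is an interactive switch actor that the player toggles with the E key.
; Its Interact function enables input on the actor for player controller 0, and E then flips IsOn and prints the new state.
; When a BP_FlowerPCharacter leaves InteractiveCollider, input is disabled again.
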(event `self.InteractiveCollider.OnComponentEndOverlap`
  (params (OverlappedComponent :type "PrimitiveComponent Object Reference") (OtherActor :type "Actor Object Reference") (OtherComp :type "PrimitiveComponent Object Reference") (OtherBodyIndex :type Integer))
  (cast `/Game/BP/BP_FlowerPCharacter` OtherActor)
  (`self.DisableInput` (`GameplayStatics.GetPlayerController` 0)))

(event `Key|E`
  (params (Key :type "Key Structure"))
  (:`Pressed`
    (bind _output_get (set `self.bIsOn` (not (`self.bIsOn`))))
    (`KismetSystemLibrary.PrintString` (`KismetStringLibrary.Conv_BoolToString` _output_get))))

(fn `Interact`
  (params (PlayerRef :type "/Game/BP/BP_FlowerPCharacter Object Reference"))
  (`self.EnableInput` (`GameplayStatics.GetPlayerController` 0)))

(fn `UserConstructionScript`
  (`parent.UserConstructionScript`))