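; BP_Light is a toggleable light zone that heals the player standing in it and turns bats around when they enter while it is lit.
; It either follows a linked BP_InteractiveSwitch, polled each Tick, or flips on a looping timer whose interval can be randomized once at BeginPlay.
; Box overlaps track the player and set its IsInLight flag, while Tick re-arms a one-shot heal timer and draws a debug box.
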(event `self.ReceiveBeginPlay`
  (if (`self.bIsAutoSwitch`)
    (if (`self.bIsRandomAuto`)
      (`KismetSystemLibrary.K2_SetTimer` null "AutoSwitchLight" (`KismetMathLibrary.RandomFloatInRange` 0.0 (`self.SwitchFrequency`)) true)
      (else
        (`KismetSystemLibrary.K2_SetTimer` null "AutoSwitchLight" (`self.SwitchFrequency`) true)))
    (else
      (bind _asbp_interactive_switch (cast `/Game/BP/Interactives/BP_InteractiveSwitch` (`self.SwitchActor`)))
      (`self.SetActiveLight` (`/Game/BP/Interactives/BP_InteractiveSwitch.bIsOn` _asbp_interactive_switch)))))

(event `self.ReceiveTick`
  (params (DeltaSeconds :type "Float (single-precision)"))
  (bind _box (`self.Box`))
  (`KismetSystemLibrary.DrawDebugBox` (`SceneComponent.K2_GetComponentLocation` _box) (`BoxComponent.BoxExtent` _box) (struct :`R` 1.0 :`G` 0.898149 :`A` 1.0) (struct) 24.0 1.0)
  (if (not (`self.bIsAutoSwitch`))
    (`self.SwitchLight`))
  (if (and (`self.bIsInLight`) (`self.bIsActive`))
    (if (not (`KismetSystemLibrary.K2_IsTimerActiveHandle` (`self.HealTimer`)))
      (bind _returnvalue (`KismetSystemLibrary.K2_SetTimerDelegate` (`|CreateDelegate` :!event `OnLightHeal`) (`self.HealFrequency`)))
      (set `self.HealTimer` _returnvalue))))

(event `OnLightHeal`
  (bind _character (`self.Character`))
  (if (and (`self.bIsInLight`) (`self.bIsActive`))
    (`/Game/BP/BP_FlowerPCharacter.AddHealth` _character (`self.HealValue`))
    (`KismetSystemLibrary.PrintString` (`KismetStringLibrary.Conv_DoubleToString` (`/Game/BP/BP_FlowerPCharacter.Health` _character)))))

(event `self.Box.OnComponentBeginOverlap`
  (params (OverlappedComponent :type "PrimitiveComponent Object Reference") (OtherActor :type "Actor Object Reference") (OtherComp :type "PrimitiveComponent Object Reference") (OtherBodyIndex :type Integer) (bFromSweep :type Boolean) (SweepResult :type "HitResult Structure (by ref)"))
  ;[1 1 1] If player in, player can heal
  (bind _asbp_flower_pcharacter (cast `/Game/BP/BP_FlowerPCharacter` OtherActor)
    (:`then`
      (bind _output_get (set `self.Character` _asbp_flower_pcharacter))
      (bind _output_get_2 (set `self.bIsInLight` true))
      (set `/Game/BP/BP_FlowerPCharacter.bIsInLight` _output_get_2 _output_get))
    (:`CastFailed`
      ;[1 0.6805 0.0317] If bat in active light, change bat dir (edit for all enemies)
      (bind _asbp_enemy_bat (cast `/Game/BP/Enemies/BP_EnemyBat` OtherActor))
      (if (`self.bIsActive`)
        (`/Game/BP/Enemies/BP_EnemyBat.UpdateFacingDirection` _asbp_enemy_bat)))))

(event `self.Box.OnComponentEndOverlap`
  (params (OverlappedComponent :type "PrimitiveComponent Object Reference") (OtherActor :type "Actor Object Reference") (OtherComp :type "PrimitiveComponent Object Reference") (OtherBodyIndex :type Integer))
  (bind _asbp_flower_pcharacter (cast `/Game/BP/BP_FlowerPCharacter` OtherActor))
  (bind _output_get (set `self.bIsInLight` false))
  (set `/Game/BP/BP_FlowerPCharacter.bIsInLight` _output_get _asbp_flower_pcharacter))

(fn `AutoSwitchLight`
  (`self.SetActiveLight` (not (`self.bIsActive`))))

(fn `LightOff`
  (bind _asbp_interactive_switch (cast `/Game/BP/Interactives/BP_InteractiveSwitch` (`self.SwitchActor`)))
  (bind _output_get (set `/Game/BP/Interactives/BP_InteractiveSwitch.bIsOn` (not (`/Game/BP/Interactives/BP_InteractiveSwitch.bIsOn` _asbp_interactive_switch)) _asbp_interactive_switch))
  (`self.SetActiveLight` _output_get))

(fn `SetActiveLight`
  (params (NewVisibility :type Boolean))
  (bind _output_get (set `self.bIsActive` NewVisibility))
  (`SceneComponent.SetVisibility` (`self.PointLight`) _output_get false))

(fn `SwitchLight`
  (bind _asbp_interactive_switch (cast `/Game/BP/Interactives/BP_InteractiveSwitch` (`self.SwitchActor`)))
  (`self.SetActiveLight` (`/Game/BP/Interactives/BP_InteractiveSwitch.bIsOn` _asbp_interactive_switch)))

(fn `UserConstructionScript`)