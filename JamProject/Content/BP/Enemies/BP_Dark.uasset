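; BP_Dark is a darkness hazard volume that damages the player character while it stays inside.
; Box overlap with BP_FlowerPCharacter sets the in-dark flag and adds a WBP_Dark overlay; leaving only clears the flag.
; While flagged, Tick restarts a short one-shot timer, apparently for OnDarkDamage, whenever it lapses and pushes DarkValue to the overlay's opacity.
; Tick also draws a debug box of the volume.
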(event `self.ReceiveBeginPlay`)

(event `self.ReceiveActorBeginOverlap`
  (params (OtherActor :type "Actor Object Reference")))

(event `self.ReceiveTick`
  (params (DeltaSeconds :type "Float (single-precision)"))
  (bind _box (`self.Box`))
  (`KismetSystemLibrary.DrawDebugBox` (`SceneComponent.K2_GetComponentLocation` _box) (`BoxComponent.BoxExtent` _box) (struct) (struct) 24.0 1.0)
  (if (`self.bIsInDark`)
    (if (not (`KismetSystemLibrary.K2_IsTimerActiveHandle` (`self.DamageTimer`)))
      (bind _returnvalue (`KismetSystemLibrary.K2_SetTimerDelegate` (`|CreateDelegate` :!event `OnDarkDamage`) 2.0))
      (set `self.DamageTimer` _returnvalue)
      (`self.UpdateDark`))))

(event `self.Box.OnComponentBeginOverlap`
  (params (OverlappedComponent :type "PrimitiveComponent Object Reference") (OtherActor :type "Actor Object Reference") (OtherComp :type "PrimitiveComponent Object Reference") (OtherBodyIndex :type Integer) (bFromSweep :type Boolean) (SweepResult :type "HitResult Structure (by ref)"))
  (bind _asbp_flower_pcharacter (cast `/Game/BP/BP_FlowerPCharacter` OtherActor))
  (set `self.Character` _asbp_flower_pcharacter)
  (set `self.bIsInDark` true)
  (bind _returnvalue (`|CreateWidget` "/Game/UI/WBP_Dark.WBP_Dark_C"))
  (bind _output_get (set `self.WBP_Dark` _returnvalue))
  (`UserWidget.AddToViewport` _output_get 0))

(event `self.Box.OnComponentEndOverlap`
  (params (OverlappedComponent :type "PrimitiveComponent Object Reference") (OtherActor :type "Actor Object Reference") (OtherComp :type "PrimitiveComponent Object Reference") (OtherBodyIndex :type Integer))
  (cast `/Game/BP/BP_FlowerPCharacter` OtherActor)
  (set `self.bIsInDark` false))

(event `OnDarkDamage`
  (if (`self.bIsInDark`)
    (`GameplayStatics.ApplyDamage` (`self.Character`) (`self.Damage`))))

(fn `UpdateDark`
  (`/Game/UI/WBP_Dark.UpdateOpacity` (`self.WBP_Dark`) (`self.DarkValue`)))

(fn `UserConstructionScript`)