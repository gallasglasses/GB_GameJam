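; Mushroom enemy that walks back and forth along the X axis, starting in a random direction and mirroring its sprite through X scale to match.
; Wall hits from anything but the player reverse it, gated by a DoOnce that resets after a short delay to avoid repeated flips.
; While the player character overlaps TargetBox, it moves faster and steers toward the player's X position.
; Death runs the parent logic, then destroys the actor.
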(event `self.ReceiveBeginPlay`
  (set `self.bIsMovingRight` (`KismetMathLibrary.RandomBool`))
  (`self.SwitchFacingDirection`))

(event `self.ReceiveTick`
  (params (DeltaSeconds :type "Float (single-precision)"))
  (bind _returnvalue_x (`KismetMathLibrary.BreakVector` (`self.K2_GetActorLocation`)))
  (bind _returnvalue_x_2 (`KismetMathLibrary.BreakVector` (`self.K2_GetActorLocation` (`self.Character Ref`))))
  (`self.AddMovementInput` (1.0 0.0 0.0) (select `bool` (`self.bIsMovingRight`) :`false` -1.0 :`true` 1.0 :!type "Float (single-precision)"))
  ;[1 1 1] Target to player
  (if (`self.bIsInTargetingRange`)
    (set `CharacterMovementComponent.MaxWalkSpeed` 80.0 (`self.CharacterMovement`))
    (if (>= (- _returnvalue_x_2 _returnvalue_x) 0.0)
      (set `self.bIsMovingRight` true)
      (else
        (set `self.bIsMovingRight` false)))
    (`self.SwitchFacingDirection`)
    (else
      (set `CharacterMovementComponent.MaxWalkSpeed` 50.0 (`self.CharacterMovement`)))))

(event `self.CapsuleComponent.OnComponentHit`
  (params (HitComponent :type "PrimitiveComponent Object Reference") (OtherActor :type "Actor Object Reference") (OtherComp :type "PrimitiveComponent Object Reference") (NormalImpulse :type "Vector Structure") (Hit :type "HitResult Structure (by ref)"))
  ;[0 0 0] If hit player, don't change dir
  (if (!= OtherActor (`GameplayStatics.GetPlayerPawn` 0))
    (if (!= (.x Hit_Normal) 0.0)
      (`/Engine/EditorBlueprintResources/StandardMacros.DoOnce` false :!label _label
        (:`Completed`
          (`self.UpdateFacingDirection`)
          ;[0.2708 0.08853 0.02859] fuu
          (`KismetSystemLibrary.Delay` 0.2)
          (`self.ResetDirChangedChecking`))))))

(event `ResetDirChangedChecking`
  (goto _label :!via `Reset`))

(event `self.TargetBox.OnComponentBeginOverlap`
  (params (OverlappedComponent :type "PrimitiveComponent Object Reference") (OtherActor :type "Actor Object Reference") (OtherComp :type "PrimitiveComponent Object Reference") (OtherBodyIndex :type Integer) (bFromSweep :type Boolean) (SweepResult :type "HitResult Structure (by ref)"))
  (bind _asbp_flower_pcharacter (cast `/Game/BP/BP_FlowerPCharacter` OtherActor))
  (set `self.bIsInTargetingRange` true)
  (set `self.Character Ref` _asbp_flower_pcharacter))

(event `self.TargetBox.OnComponentEndOverlap`
  (params (OverlappedComponent :type "PrimitiveComponent Object Reference") (OtherActor :type "Actor Object Reference") (OtherComp :type "PrimitiveComponent Object Reference") (OtherBodyIndex :type Integer))
  (cast `/Game/BP/BP_FlowerPCharacter` OtherActor)
  (set `self.bIsInTargetingRange` false))

(fn `Died`
  (`parent.Died`)
  (`self.K2_DestroyActor`))

(fn `SwitchFacingDirection`
  (bind (_returnvalue_x _returnvalue_y _returnvalue_z) (`KismetMathLibrary.BreakVector` (`SceneComponent.K2_GetComponentScale` (`self.Sprite`))))
  (`SceneComponent.SetWorldScale3D` (`self.Sprite`) (`KismetMathLibrary.MakeVector` (* (`KismetMathLibrary.Abs` _returnvalue_x) (select `bool` (`self.bIsMovingRight`) :`false` 1.0 :`true` -1.0 :!type "Float (single-precision)")) _returnvalue_y _returnvalue_z)))

(fn `UpdateFacingDirection`
  (set `self.bIsMovingRight` (not (`self.bIsMovingRight`)))
  (`self.SwitchFacingDirection`))

(fn `UserConstructionScript`
  (`parent.UserConstructionScript`))