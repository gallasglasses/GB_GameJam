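; Big bloated 2D enemy that walks sideways, flips on hitting non-player obstacles, and turns toward the player inside its target box.
; It is hurt through a light puzzle: when all linked BP_Lights are active, it switches them off, takes about a third of its default health, and advances a wave counter.
; From the first wave on, a looping timer spawns bullets at its sphere, aimed using a point above it.
; UpdateFlipbook selects animations from movement, damage and death state.
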(event `self.ReceiveBeginPlay`
  (set `self.bIsMovingRight` (`KismetMathLibrary.RandomBool`))
  (`self.SwitchFacingDirection`)
  (`KismetSystemLibrary.K2_SetTimer` null "MakeShot" 3.0 true))

(event `self.ReceiveTick`
  (params (DeltaSeconds :type "Float (single-precision)"))
  (bind _returnvalue_x (`KismetMathLibrary.BreakVector` (`self.K2_GetActorLocation`)))
  (bind _lights (`self.Lights`))
  (bind _returnvalue_x_2 (`KismetMathLibrary.BreakVector` (`self.K2_GetActorLocation` (`self.Character Ref`))))
  (`self.AddMovementInput` (1.0 0.0 0.0) (select `bool` (`self.bIsMovingRight`) :`false` -1.0 :`true` 1.0 :!type "Float (single-precision)"))
  ;[1 1 1] Target to player
  (if (`self.bIsInTargetingRange`)
    (if (>= (- _returnvalue_x_2 _returnvalue_x) 0.0)
      (set `self.bIsMovingRight` true)
      (else
        (set `self.bIsMovingRight` false)))
    (`self.SwitchFacingDirection`))
  (bind _bisalllighton (`self.IsAllLightOn`))
  (if _bisalllighton
    (set `self.LightCount` 0)
    (for _index (range (+ (`KismetArrayLibrary.Array_Length` _lights) 1))
      (bind _asbp_light (cast `/Game/BP/LightingCondition/BP_Light` (`|GetArrayItem` _lights _index)))
      (`/Game/BP/LightingCondition/BP_Light.LightOff` _asbp_light))
    (`GameplayStatics.ApplyDamage` self (/ (`self.DefaultHealth`) 2.9))
    (bind _result (`/Engine/EditorBlueprintResources/StandardMacros.IncrementFloat` (`self.WaveCount`))
      (:`  `
        (set `self.WaveCount` _result)
        (`KismetSystemLibrary.PrintString` (`KismetStringLibrary.Conv_DoubleToString` (`self.WaveCount`)))))))

(event `self.CapsuleComponent.OnComponentHit`
  (params (HitComponent :type "PrimitiveComponent Object Reference") (OtherActor :type "Actor Object Reference") (OtherComp :type "PrimitiveComponent Object Reference") (NormalImpulse :type "Vector Structure") (Hit :type "HitResult Structure (by ref)"))
  ;[0 0 0] If hit player, don't change dir
  (if (!= OtherActor (`GameplayStatics.GetPlayerPawn` 0))
    (if (!= (.x Hit_Normal) 0.0)
      (`/Engine/EditorBlueprintResources/StandardMacros.DoOnce` false :!label _label
        (:`Completed`
          (`self.UpdateFacingDirection`)
          ;[0.2708 0.08853 0.02859] fuu
          (`KismetSystemLibrary.Delay` 0.2)
          (`self.ResetDirChangedChecking`))))))

(event `ResetDirChangedChecking`
  (goto _label :!via `Reset`))

(event `self.TargetBox.OnComponentBeginOverlap`
  (params (OverlappedComponent :type "PrimitiveComponent Object Reference") (OtherActor :type "Actor Object Reference") (OtherComp :type "PrimitiveComponent Object Reference") (OtherBodyIndex :type Integer) (bFromSweep :type Boolean) (SweepResult :type "HitResult Structure (by ref)"))
  (bind _asbp_flower_pcharacter (cast `/Game/BP/BP_FlowerPCharacter` OtherActor))
  (set `self.bIsInTargetingRange` true)
  (set `self.Character Ref` _asbp_flower_pcharacter))

(event `self.TargetBox.OnComponentEndOverlap`
  (params (OverlappedComponent :type "PrimitiveComponent Object Reference") (OtherActor :type "Actor Object Reference") (OtherComp :type "PrimitiveComponent Object Reference") (OtherBodyIndex :type Integer))
  (cast `/Game/BP/BP_FlowerPCharacter` OtherActor)
  (set `self.bIsInTargetingRange` false))

(fn `Died`
  (`parent.Died`)
  (`self.K2_DestroyActor`))

(fn `IsAllLightOn`
  (returns (bIsAllLightOn :type Boolean))
  (bind _lights (`self.Lights`))
  (bind _returnvalue (`KismetArrayLibrary.Array_Length` _lights))
  (set `self.LightCount` 0)
  (for _index (range (+ _returnvalue 1))
    (bind _asbp_light (cast `/Game/BP/LightingCondition/BP_Light` (`|GetArrayItem` _lights _index)))
    (if (`/Game/BP/LightingCondition/BP_Light.bIsActive` _asbp_light)
      (set `self.LightCount` (+ (`self.LightCount`) 1))
      (else
        (set `self.LightCount` 0))))
  (return (== _returnvalue (`self.LightCount`))))

(fn `MakeShot`
  (bind _projectile (`self.Projectile`))
  (bind _returnvalue (`SceneComponent.K2_GetComponentLocation` (`self.Sphere`)))
  (bind (_returnvalue_x _returnvalue_y _returnvalue_z) (`KismetMathLibrary.BreakVector` (`SceneComponent.K2_GetComponentLocation` (`self.Sphere`))))
  (bind (_bblockinghit _binitialoverlap _time _distance _location _impactpoint _normal _impactnormal _physmat _hitactor _hitcomponent _hitbonename _hititem _faceindex _tracestart _traceend) (`GameplayStatics.BreakHitResult` (`GameplayStatics.MakeHitResult` false false 0.0 0.0 (0.0 0.0 0.0) (0.0 0.0 0.0) (0.0 0.0 1.0) (0.0 0.0 1.0) null null null "None" 0 0 _returnvalue (`KismetMathLibrary.MakeVector` _returnvalue_x _returnvalue_y (+ _returnvalue_z 100.0)))))
  (if (>= (`self.WaveCount`) 1.0)
    (bind _returnvalue_2 (`|SpawnActorFromClass` "/Game/BP/Enemies/BP_Bullet.BP_Bullet_C" (`SceneComponent.K2_GetComponentToWorld` (`self.Sphere`)) "Undefined" "OverrideRootScale" self null))
    (set `self.Projectile` _returnvalue_2)
    (if _bblockinghit
      (set `self.Direction` (- _impactpoint _returnvalue))
      (else
        (set `self.Direction` (- _traceend _returnvalue))))
    (bind _asbp_bullet (cast `/Game/BP/Enemies/BP_Bullet` _projectile))
    (set `/Game/BP/Enemies/BP_Bullet.Dir` (`self.Direction`) _asbp_bullet)
    (`self.SetOwner` _projectile (`self.GetOwner`))))

(fn `SwitchFacingDirection`
  (bind (_returnvalue_x _returnvalue_y _returnvalue_z) (`KismetMathLibrary.BreakVector` (`SceneComponent.K2_GetComponentScale` (`self.Sprite`))))
  (`SceneComponent.SetWorldScale3D` (`self.Sprite`) (`KismetMathLibrary.MakeVector` (* (`KismetMathLibrary.Abs` _returnvalue_x) (select `bool` (`self.bIsMovingRight`) :`false` 1.0 :`true` -1.0 :!type "Float (single-precision)")) _returnvalue_y _returnvalue_z)))

(fn `UpdateFacingDirection`
  (set `self.bIsMovingRight` (not (`self.bIsMovingRight`)))
  (`self.SwitchFacingDirection`))

(fn `UpdateFlipbook`
  (bind (_returnvalue_x _returnvalue_y _returnvalue_z) (`KismetMathLibrary.BreakVector` (`self.GetVelocity`)))
  (if (`self.bIsDead`)
    (set `self.MovementState` "NewEnumerator6")
    (elif (`self.bIsDamage`)
      (set `self.MovementState` "NewEnumerator7")
      (else
        (set `self.MovementState` (select `bool` (!= (`KismetMathLibrary.VSize` (`self.GetVelocity`)) 0.0) :`false` "NewEnumerator0" :`true` (select `bool` (`NavMovementComponent.IsFalling` (`self.CharacterMovement`)) :`false` "NewEnumerator1" :`true` (select `bool` (<= _returnvalue_z 0.0) :`false` "NewEnumerator2" :`true` "NewEnumerator3" :!type "/Game/BP/E_CharacterMovement Enum")))))))
  (`PaperFlipbookComponent.SetFlipbook` (`self.Sprite`) (select `/Game/BP/E_CharacterMovement` (`self.MovementState`) :`NewEnumerator0` (`self.FB_Idle`) :`NewEnumerator1` (`self.FB_Run`) :`NewEnumerator2` (`self.FB_Jump`) :`NewEnumerator3` (`self.FB_Fall`) :`NewEnumerator5` (`self.FB_Appearing`) :`NewEnumerator6` (`self.FB_Desappearing`) :`NewEnumerator7` (`self.FB_Hit`)))
  (if (or (or (`|EnumEquality` (`self.MovementState`) "NewEnumerator5") (`|EnumEquality` (`self.MovementState`) "NewEnumerator6")) (`|EnumEquality` (`self.MovementState`) "NewEnumerator7"))
    (`PaperFlipbookComponent.SetLooping` (`self.Sprite`) false)))

(fn `UserConstructionScript`
  (`parent.UserConstructionScript`))