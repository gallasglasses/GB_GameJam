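; BP_Bullet is an enemy projectile that damages the flower player character on impact.
; On spawn it sets its ProjectileMovement velocity from the local-space Dir vector and starts a configurable lifespan.
; A sphere hit stops movement, applies Damage to the cast player reference and destroys the bullet.
; Hits on other actors print the actor's name, and the damage target is then the failed cast result.
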(event `self.ReceiveBeginPlay`
  (`ProjectileMovementComponent.SetVelocityInLocalSpace` (`self.ProjectileMovement`) (`self.Dir`))
  (`self.SetLifeSpan` (`self.In Lifespan`)))

(event `self.Sphere.OnComponentHit`
  (params (HitComponent :type "PrimitiveComponent Object Reference") (OtherActor :type "Actor Object Reference") (OtherComp :type "PrimitiveComponent Object Reference") (NormalImpulse :type "Vector Structure") (Hit :type "HitResult Structure (by ref)"))
  (`MovementComponent.StopMovementImmediately` (`self.ProjectileMovement`))
  (bind _asbp_flower_pcharacter (cast `/Game/BP/BP_FlowerPCharacter` OtherActor)
    (:`then`
      _)
    (:`CastFailed`
      (`KismetSystemLibrary.PrintString` (`KismetSystemLibrary.GetDisplayName` OtherActor))))
  (`GameplayStatics.ApplyDamage` _asbp_flower_pcharacter (`self.Damage`))
  (`self.K2_DestroyActor`))

(fn `UserConstructionScript`)